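; BP_Cube1 is a moving cube actor that shuttles along the X axis and jumps to a fixed position when hit by a first-person projectile.
; Tick moves it from the static mesh's transform along the normalized Direction, scaled by Speed and delta time.
; A Delay inside Tick feeds a FlipFlop that reverses Direction about every six seconds.
; The Hit event filters for FirstPersonProjectile, then sets the hard-coded location without sweeping.
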(event `self.ReceiveHit`
  (params (MyComp :type "PrimitiveComponent Object Reference") (Other :type "Actor Object Reference") (OtherComp :type "PrimitiveComponent Object Reference") (bSelfMoved :type Boolean) (HitLocation :type "Vector Structure") (HitNormal :type "Vector Structure") (NormalImpulse :type "Vector Structure") (Hit :type "HitResult Structure (by ref)"))
  (cast `/Game/FirstPersonBP/Blueprints/FirstPersonProjectile` Other)
  (`self.K2_SetActorLocation` (820.0 -500.0 290.0)))

(event `self.ReceiveTick`
  (params (DeltaSeconds :type "Float (single-precision)"))
  ;[1 1 1] 移动
  (`self.K2_SetActorTransform` (`KismetMathLibrary.MakeTransform` (+ (.location (`SceneComponent.K2_GetComponentToWorld` (`self.StaticMeshComponent`))) (* (`KismetMathLibrary.Normal` (`self.Direction`) 3.0) (* (`self.Speed`) (`GameplayStatics.GetWorldDeltaSeconds`)))) (.rotation (`SceneComponent.K2_GetComponentToWorld` (`self.StaticMeshComponent`))) (.scale (`SceneComponent.K2_GetComponentToWorld` (`self.StaticMeshComponent`)))))
  ;;[1 1 1] 反向
  (`KismetSystemLibrary.Delay` 6.0)
  (`/Engine/EditorBlueprintResources/StandardMacros.FlipFlop`
    (:`A`
      (set `self.Direction` (10.0 0.0 0.0)))
    (:`B`
      (set `self.Direction` (-10.0 0.0 0.0)))))

(fn `UserConstructionScript`)